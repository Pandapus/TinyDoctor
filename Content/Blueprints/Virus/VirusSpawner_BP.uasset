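; Virus spawner actor that populates the area around itself with Virus_BP actors when play begins.
; SpawnVirus places NumberToSpawn viruses at random navigable points around the spawner, each with a random yaw.
; The spawn radius grows sublinearly with the count through a power curve, so larger groups spread wider.
; Each virus receives a reference to the spawner and is stored in VirusArray.
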(event EventBeginPlay
  (CallFunction|SpawnVirus))

(fn ConstructionScript)

(fn SpawnVirus
  (for _index (range 1 (Variables|Default|GetnumberToSpawn))
    (bind _returnvalue (Game|SpawnActorfromClass "/Game/Blueprints/Virus/Virus_BP.Virus_BP_C" (Math|Transform|MakeTransform (Class|NavigationSystem|GetRandomPointinNavigableRadius (Transformation|GetActorLocation) (Math|Float|Power (* (Math|Conversions|ToFloat(Integer) (Variables|Default|GetnumberToSpawn)) 4e+01) 0.75)) (Math|Rotator|MakeRotator 0.0 0.0 (Math|Random|RandomFloatinRange -1.8e+02 1.8e+02))) "AdjustIfPossibleButAlwaysSpawn" 0 self 0))
    (Utilities|Array|Add (Variables|Default|GetvirusArray) _returnvalue)))