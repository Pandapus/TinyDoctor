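; Level gateway actor that moves the player to another level when they walk into it.
; On box overlap by a PlayerCharacter, it copies the player's health and ammo into the StandardGameInstance so they persist across the load.
; It then opens the level named by its NameOfTargetLevel variable.
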(event OnComponentBeginOverlap(Box)
  (params (OverlappedComponent :type Primitive%20Component%20Object%20Reference) (OtherActor :type Actor%20Object%20Reference) (OtherComp :type Primitive%20Component%20Object%20Reference) (OtherBodyIndex :type Integer) (bFromSweep :type Boolean) (SweepResult :type Hit%20Result%20Structure%20%28by%20ref%29))
  (if (Utilities|ClassIsChildOf (Utilities|GetClass OtherActor) "/Script/TinyDoctorTest.PlayerCharacter")
    (bind _asplayer_character (Utilities|Casting|CastToPlayerCharacter OtherActor))
    (bind _asstandard_game_instance (Utilities|Casting|CastToStandardGameInstance (Game|GetGameInstance)))
    (Variables|/Script/TinyDoctorTest.StandardGameInstance|SetplayerHealth _asstandard_game_instance (Class|Unit|GetHealth _asplayer_character))
    (Variables|/Script/TinyDoctorTest.StandardGameInstance|SetplayerAmmo _asstandard_game_instance (Class|PlayerCharacter|GetAmmo _asplayer_character))
    (Game|OpenLevel(byName) (Utilities|String|StringToName (Variables|Default|GetNameOfTargetLevel)))))

(fn ConstructionScript)