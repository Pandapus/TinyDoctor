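; Health pickup Blueprint that adds health to the player character when an actor overlaps it.
; The overlap event calls the parent handler, casts player 0's character to PlayerCharacter and passes it to IncreaseHealth with a fixed amount.
; The overlapping actor is never checked, so any overlap heals the player.
; IncreaseHealth adds to Health without clamping, and this graph does not destroy the pickup.
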(event EventBeginPlay)

(event Collision|EventActorBeginOverlap
  (params (OtherActor :type Actor%20Object%20Reference))
  (|CallParentFunction OtherActor)
  (bind _asplayer_character (Utilities|Casting|CastToPlayerCharacter (Game|GetPlayerCharacter 0)))
  (CallFunction|IncreaseHealth 1.0 _asplayer_character))

(event EventTick
  (params (DeltaSeconds :type Float%20%28single-precision%29))
  (|CallParentFunction DeltaSeconds))

(fn ConstructionScript
  (|CallParentFunction))

(fn IncreaseHealth
  (params (Amount :type Float%20%28single-precision%29) (UnitReference :type Unit%20Object%20Reference))
  (bind _output_get (LocalVariables|SetLocalPlayerRef UnitReference))
  (Variables|/Script/TinyDoctorTest.Unit|Sethealth UnitReference (+ (Variables|/Script/TinyDoctorTest.Unit|Gethealth _output_get) Amount)))