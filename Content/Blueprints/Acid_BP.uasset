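; Acid hazard actor that deals continuous damage to any Unit standing inside its Cube volume.
; Cube overlap events add and remove units in the OverlappingUnits list.
; Each Tick calls ReduceHealth on every listed unit with DamagePerSecond scaled by delta time.
; Units are dropped from the list when ReduceHealth returns true or they become invalid, removed during the loop itself.
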(event OnComponentBeginOverlap(Cube)
  (params (OverlappedComponent :type Primitive%20Component%20Object%20Reference) (OtherActor :type Actor%20Object%20Reference) (OtherComp :type Primitive%20Component%20Object%20Reference) (OtherBodyIndex :type Integer) (bFromSweep :type Boolean) (SweepResult :type Hit%20Result%20Structure%20%28by%20ref%29))
  (if (Utilities|ClassIsChildOf (Utilities|GetClass OtherActor) "/Script/TinyDoctorTest.Unit")
    (bind _asunit (Utilities|Casting|CastToUnit OtherActor))
    (Utilities|Array|Add (Variables|Default|GetOverlapping%20Units) _asunit)))

(event OnComponentEndOverlap(Cube)
  (params (OverlappedComponent :type Primitive%20Component%20Object%20Reference) (OtherActor :type Actor%20Object%20Reference) (OtherComp :type Primitive%20Component%20Object%20Reference) (OtherBodyIndex :type Integer))
  (if (Utilities|ClassIsChildOf (Utilities|GetClass OtherActor) "/Script/TinyDoctorTest.Unit")
    (bind _asunit (Utilities|Casting|CastToUnit OtherActor))
    (Utilities|Array|RemoveItem (Variables|Default|GetOverlapping%20Units) _asunit)))

(event EventTick
  (params (DeltaSeconds :type Float%20%28single-precision%29))
  ;[1 1 1] Damage every unit
  (for _array_element (Variables|Default|GetOverlapping%20Units)
    (if (Utilities|IsValid _array_element)
      (bind _returnvalue (Class|Unit|ReduceHealth _array_element (* DeltaSeconds (Variables|Default|GetDamage%20Per%20Second))))
      (if _returnvalue
        (Utilities|Array|RemoveItem (Variables|Default|GetOverlapping%20Units) _array_element))
      (else
        (Utilities|Array|RemoveItem (Variables|Default|GetOverlapping%20Units) _array_element)))))

(fn ConstructionScript)