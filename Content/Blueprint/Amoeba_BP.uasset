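; Amoeba enemy that deals contact damage to the player character and knocks it back.
; On capsule hit it subtracts health and launches the player away, with TouchDamageKnockbackVertical scaling XY and TouchDamageKnockbackHorizontal setting Z, opposite to their names.
; A player at zero health or below is destroyed; otherwise a delay flag blocks repeat hits until the cooldown ends, then the amoeba moves toward that player.
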(event OnComponentHit(CapsuleComponent)
  (params (HitComponent :type Primitive%20Component%20Object%20Reference) (OtherActor :type Actor%20Object%20Reference) (OtherComp :type Primitive%20Component%20Object%20Reference) (NormalImpulse :type Vector :default "0, 0, 0") (Hit :type Hit%20Result%20Structure%20%28by%20ref%29))
  (if (not (Variables|Default|Getdelayed self))
    (if (Utilities|ClassIsChildOf (Utilities|GetClass OtherActor) "/Script/TinyDoctorTest.PlayerCharacter")
      (bind _asplayer_character (Utilities|Casting|CastToPlayerCharacter OtherActor))
      (bind _output_get (Variables|/Script/TinyDoctorTest.Unit|Sethealth _asplayer_character (- (Variables|/Script/TinyDoctorTest.Unit|Gethealth _asplayer_character) (Variables|Default|GettouchDamage))))
      (Character|LaunchCharacter _asplayer_character (Math|Vector|MakeVector (.X (Math|Vector2D|BreakVector2D (* (Math|Vector2D|MakeVector2D (.X (Math|Vector|BreakVector (Math|Vector|Normalize (- (Transformation|GetActorLocation _asplayer_character) (Transformation|GetActorLocation))))) (.Y (Math|Vector|BreakVector (Math|Vector|Normalize (- (Transformation|GetActorLocation _asplayer_character) (Transformation|GetActorLocation)))))) (Variables|Default|GettouchDamageKnockbackVertical)))) (.Y (Math|Vector2D|BreakVector2D (* (Math|Vector2D|MakeVector2D (.X (Math|Vector|BreakVector (Math|Vector|Normalize (- (Transformation|GetActorLocation _asplayer_character) (Transformation|GetActorLocation))))) (.Y (Math|Vector|BreakVector (Math|Vector|Normalize (- (Transformation|GetActorLocation _asplayer_character) (Transformation|GetActorLocation)))))) (Variables|Default|GettouchDamageKnockbackVertical)))) (Variables|Default|GettouchDamageKnockbackHorizontal)) true true)
      (Variables|Default|Setdelayed true)
      (if (<= _output_get 0.0)
        (Actor|DestroyActor _asplayer_character)
        (else
          (Utilities|FlowControl|Delay (Variables|Default|GetdelayDuration))
          (Variables|Default|Setdelayed self false)
          (AI|Navigation|SimpleMovetoActor (Pawn|GetController) _asplayer_character))))))

(event EventBeginPlay)

(event Collision|EventActorBeginOverlap
  (params (OtherActor :type Actor%20Object%20Reference)))

(event EventTick
  (params (DeltaSeconds :type Float%20%28single-precision%29)))

(fn ConstructionScript)