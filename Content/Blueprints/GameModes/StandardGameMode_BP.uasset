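; Standard game mode that handles pausing and the win and lose screens.
; On BeginPlay it creates and caches the pause menu widget and spawns an AimPlane actor at the world origin.
; PauseGame toggles the paused state, adding or removing the cached menu.
; GameOver and GameWon each pause the game and show a newly created result widget.
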(event EventBeginPlay
  ;[1 1 1] Begin Play
  ;[1 1 1] Create Pause Menu Reference
  (bind _returnvalue (UserInterface|CreateWidget "/Game/UI/PauseMenu_UI.PauseMenu_UI_C" (Game|GetPlayerController 0)))
  (Variables|Default|SetPause%20Menu%20Reference _returnvalue)
  ;[1 1 1] Spawn AimPlane
  (Game|SpawnActorfromClass "/Game/Blueprints/Player/AimPlane_BP.AimPlane_BP_C" (Math|Transform|MakeTransform "0, 0, 0") "AlwaysSpawn" 0 0))

(event EventPauseGame
  ;[1 1 1] Pause Game
  (if (Game|IsGamePaused)
    (Game|SetGamePaused false)
    (Widget|RemovefromParent (Variables|Default|GetPause%20Menu%20Reference))
    (else
      (Game|SetGamePaused true)
      (UserInterface|Viewport|AddtoViewport (Variables|Default|GetPause%20Menu%20Reference) 0))))

(event EventGameOver
  ;[1 1 1] Game Over
  (Game|SetGamePaused true)
  (bind _returnvalue (UserInterface|CreateWidget "/Game/UI/GameOver_UI.GameOver_UI_C" (Game|GetPlayerController 0)))
  (UserInterface|Viewport|AddtoViewport _returnvalue 0))

(event EventGameWon
  ;[1 1 1] Game Won
  (Game|SetGamePaused true)
  (bind _returnvalue (UserInterface|CreateWidget "/Game/UI/GameWon_UI.GameWon_UI_C" (Game|GetPlayerController 0)))
  (UserInterface|Viewport|AddtoViewport _returnvalue 0))

(fn ConstructionScript)