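; Boss tentacle actor that reaches for the player within 1500 units and deals damage with knockback when it hits a player character.
; Tick either calls AttackPlayer, which interpolates TentakelEnd toward a point just behind the player while turning it to face them, or runs idle mode.
; Idle mode eases TentakelEnd back to its BeginPlay position with a sine-wave vertical bob.
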(event EventBeginPlay
  (bind _asplayer_bp (Utilities|Casting|CastToPlayer_BP (Game|GetPlayerCharacter 0)))
  (Variables|Default|SetPlayerReference _asplayer_bp)
  (Variables|Default|SetTentakelStartingPoint (Transformation|GetWorldLocation (Variables|Default|GetTentakelEnd))))

(event Collision|EventActorBeginOverlap
  (params (OtherActor :type Actor%20Object%20Reference)))

(event EventTick
  (params (DeltaSeconds :type Float%20%28single-precision%29))
  (if (<= (Transformation|GetDistanceTo (Variables|Default|GetPlayerReference)) 1.5e+03)
    (CallFunction|AttackPlayer DeltaSeconds)
    (else
      ;[1 1 1] Idle mode
      (Transformation|SetRelativeLocation (Variables|Default|GetTentakelEnd) (+ (Math|Transform|InverseTransformLocation (Transformation|GetActorTransform) (Math|Interpolation|VInterpTo (Transformation|GetWorldLocation (Variables|Default|GetTentakelEnd)) (Variables|Default|GetTentakelStartingPoint) (Utilities|Time|GetWorldDeltaSeconds) 1.0)) (* "0.000000,0.000000,1.000000" (* (Math|Trig|Sin(Radians) (* (Utilities|Time|GetTimeSeconds) 4.0)) 3.0))) false false))))

(event Collision|EventHit
  (params (MyComp :type Primitive%20Component%20Object%20Reference) (Other :type Actor%20Object%20Reference) (OtherComp :type Primitive%20Component%20Object%20Reference) (bSelfMoved :type Boolean) (HitLocation :type Vector :default "0, 0, 0") (HitNormal :type Vector :default "0, 0, 0") (NormalImpulse :type Vector :default "0, 0, 0") (Hit :type Hit%20Result%20Structure%20%28by%20ref%29))
  (if (Utilities|ClassIsChildOf (Utilities|GetClass Other) "/Script/TinyDoctorTest.PlayerCharacter")
    (bind _asplayer_character (Utilities|Casting|CastToPlayerCharacter Other))
    (Class|Unit|TakeDamagewithKnockback _asplayer_character 0.02 (Transformation|GetActorLocation) 7.5e+02 7.5e+02)
    (Utilities|FlowControl|Delay 1.0)))

(fn ConstructionScript)

(fn AttackPlayer
  (params (DeltaTime :type Float%20%28single-precision%29))
  (bind _playerreference (Variables|Default|GetPlayerReference))
  (bind _returnvalue (Transformation|GetActorLocation _playerreference))
  ;[1 1 1] Angriper spilleren
  (Transformation|SetWorldLocationAndRotation (Variables|Default|GetTentakelEnd) (Math|Interpolation|VInterpTo (Transformation|GetWorldLocation (Variables|Default|GetTentakelEnd)) (+ (* (* (Transformation|GetActorForwardVector _playerreference) -1.0) 2e+02) _returnvalue) DeltaTime 3.0) (Math|Rotator|FindLookatRotation (Transformation|GetWorldLocation (Variables|Default|GetTentakelEnd)) _returnvalue) false false))