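; Projectile actor that damages Unit actors it hits.
; On BeginPlay it launches its Sphere along the actor's forward vector with a Speed-scaled force applied as an acceleration change, ignoring mass.
; When the Sphere hits a Unit, it subtracts a fixed point of Health and destroys that Unit once Health runs out.
; The projectile destroys itself on impact, whether or not it struck a Unit.
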(event OnComponentHit(Sphere)
  (params (HitComponent :type Primitive%20Component%20Object%20Reference) (OtherActor :type Actor%20Object%20Reference) (OtherComp :type Primitive%20Component%20Object%20Reference) (NormalImpulse :type Vector :default "0, 0, 0") (Hit :type Hit%20Result%20Structure%20%28by%20ref%29))
  (if (Utilities|ClassIsChildOf (Utilities|GetClass OtherActor) "/Script/TinyDoctorTest.Unit")
    (bind _asunit (Utilities|Casting|CastToUnit OtherActor))
    (bind _output_get (Variables|/Script/TinyDoctorTest.Unit|Sethealth _asunit (- (Variables|/Script/TinyDoctorTest.Unit|Gethealth _asunit) 1.0)))
    (if (<= _output_get 0.0)
      (Actor|DestroyActor _asunit)))
  (Actor|DestroyActor))

(event EventBeginPlay
  (Physics|AddForce (Variables|Default|GetSphere) (* (Transformation|GetActorForwardVector) (* (Variables|Default|GetSpeed) 1e+03)) "None" (Class|KismetSystemLibrary|MakeLiteralBool true)))

(event Collision|EventActorBeginOverlap
  (params (OtherActor :type Actor%20Object%20Reference)))

(event EventTick
  (params (DeltaSeconds :type Float%20%28single-precision%29)))

(fn ConstructionScript)