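; Amoeba enemy character that hurts the player on contact and scatters ammo pickups when destroyed.
; A capsule hit on a PlayerCharacter deals touch damage with knockback away from the amoeba's location, then after a delay orders its controller to move toward that player.
; On destruction it spawns a random number of ammo pickups around itself and launches each with a randomized upward force.
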(event OnComponentHit(CapsuleComponent)
  (params (HitComponent :type Primitive%20Component%20Object%20Reference) (OtherActor :type Actor%20Object%20Reference) (OtherComp :type Primitive%20Component%20Object%20Reference) (NormalImpulse :type Vector :default "0, 0, 0") (Hit :type Hit%20Result%20Structure%20%28by%20ref%29))
  (if (Utilities|ClassIsChildOf (Utilities|GetClass OtherActor) "/Script/TinyDoctorTest.PlayerCharacter")
    (bind _asplayer_character (Utilities|Casting|CastToPlayerCharacter OtherActor))
    (Class|Unit|TakeDamagewithKnockback _asplayer_character (Variables|Default|GettouchDamage) (Transformation|GetActorLocation) 7.5e+02 7.5e+02)
    (Utilities|FlowControl|Delay (Variables|Default|GetdelayDuration))
    (AI|Navigation|SimpleMovetoActor (Pawn|GetController) OtherActor)))

(event EventBeginPlay)

(event Collision|EventActorBeginOverlap
  (params (OtherActor :type Actor%20Object%20Reference)))

(event EventTick
  (params (DeltaSeconds :type Float%20%28single-precision%29)))

(event EventDestroyed
  (bind _returnvalue (Transformation|GetActorLocation))
  (bind (_x _y _z) (Math|Vector|BreakVector _returnvalue))
  (for _index (range 0 (Math|Random|RandomIntegerinRange 0 4))
    (bind _returnvalue_2 (Game|SpawnActorfromClass "/Game/Blueprints/Items/PickUp_BP_Ammo.PickUp_BP_Ammo_C" (Math|Conversions|ToTransform(Vector) (Math|Vector|MakeVector (+ _x (Math|Random|RandomFloatinRange -1e+02 1e+02)) (+ _y (Math|Random|RandomFloatinRange -1e+02 1e+02)) _z)) "AlwaysSpawn" 0 0))
    (Physics|AddForce (Variables|/Game/Blueprints/Items/PickUp_BP.PickUp_BP_C|GetSphereMesh _returnvalue_2) (* (Math|Vector|MakeVector (Math|Random|RandomFloatinRange -5e+02 5e+02) (Math|Random|RandomFloatinRange -5e+02 5e+02) 5e+02) 1e+02) "None" true)))

(fn ConstructionScript)