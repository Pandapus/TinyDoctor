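; Ammo pickup Blueprint that gives the player one ammo when an actor overlaps it.
; On overlap it runs the parent handler, casts player 0's character to PlayerCharacter and calls IncreaseAmmo to add to its Ammo.
; The overlapping actor is never checked, so any overlap credits the player, and any removal of the pickup is left outside this Blueprint.
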(event EventBeginPlay)

(event Collision|EventActorBeginOverlap
  (params (OtherActor :type Actor%20Object%20Reference))
  (|CallParentFunction OtherActor)
  (bind _asplayer_character (Utilities|Casting|CastToPlayerCharacter (Game|GetPlayerCharacter 0)))
  (CallFunction|IncreaseAmmo 1 _asplayer_character))

(event EventTick
  (params (DeltaSeconds :type Float%20%28single-precision%29))
  (|CallParentFunction DeltaSeconds))

(fn ConstructionScript
  (|CallParentFunction))

(fn IncreaseAmmo
  (params (Amount :type Integer) (PlayerReference :type Player%20Character%20Object%20Reference))
  (bind _output_get (Variables|Default|SetPlayerRef PlayerReference))
  (Variables|/Script/TinyDoctorTest.PlayerCharacter|Setammo PlayerReference (+ (Variables|/Script/TinyDoctorTest.PlayerCharacter|Getammo _output_get) Amount)))