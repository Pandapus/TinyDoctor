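; Projectile actor that launches along its forward vector on spawn and damages units it hits.
; BeginPlay applies a mass-independent force to the Sphere component, scaled by Speed, and plays a shoot cue.
; On a Sphere hit, a Unit loses health with horizontal and vertical knockback plus a hit sound, and any hit destroys the projectile.
; Both sounds play at the world origin rather than at the projectile.
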(event OnComponentHit(Sphere)
  (params (HitComponent :type Primitive%20Component%20Object%20Reference) (OtherActor :type Actor%20Object%20Reference) (OtherComp :type Primitive%20Component%20Object%20Reference) (NormalImpulse :type Vector :default "0, 0, 0") (Hit :type Hit%20Result%20Structure%20%28by%20ref%29))
  (if (Utilities|ClassIsChildOf (Utilities|GetClass OtherActor) "/Script/TinyDoctorTest.Unit")
    (bind _asunit (Utilities|Casting|CastToUnit OtherActor))
    (Audio|SpawnSoundatLocation "/Game/Audio/Hit.Hit" "0, 0, 0")
    (Class|Unit|ReduceHealth _asunit 1.0 self 5e+02 5e+02))
  (Actor|DestroyActor))

(event EventBeginPlay
  (Physics|AddForce (Variables|Default|GetSphere) (* (Transformation|GetActorForwardVector) (* (Variables|Default|GetSpeed) 1e+03)) "None" (Class|KismetSystemLibrary|MakeLiteralBool true))
  (Audio|PlaySoundatLocation "/Game/Audio/ShootCue.ShootCue" "0, 0, 0"))

(fn ConstructionScript)