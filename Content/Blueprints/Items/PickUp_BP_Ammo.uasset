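; Ammo pickup that refills the player's ammo when the player walks into it.
; A sphere overlap checks that the other actor's class derives from PlayerCharacter and that the stored player reference is below max ammo.
; It then calls DestroySelf and adds RefillAmount through ChangeAmmo, so the pickup stays in place when ammo is full.
; BeginPlay and construction only call the parent.
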(event OnComponentBeginOverlap(Sphere)
  (params (OverlappedComponent :type Primitive%20Component%20Object%20Reference) (OtherActor :type Actor%20Object%20Reference) (OtherComp :type Primitive%20Component%20Object%20Reference) (OtherBodyIndex :type Integer) (bFromSweep :type Boolean) (SweepResult :type Hit%20Result%20Structure%20%28by%20ref%29))
  (bind _player_reference (Variables|Default|GetPlayer%20Reference))
  (if (Utilities|ClassIsChildOf (Utilities|GetClass OtherActor) "/Script/TinyDoctorTest.PlayerCharacter")
    (if (< (Class|PlayerCharacter|GetAmmo _player_reference) (Class|PlayerCharacter|GetMaxAmmo _player_reference))
      (CallFunction|DestroySelf)
      (Class|PlayerCharacter|ChangeAmmo _player_reference (Variables|Default|GetRefillAmount)))))

(event EventTick
  (params (DeltaSeconds :type Float%20%28single-precision%29)))

(event EventBeginPlay
  (|CallParentFunction))

(fn ConstructionScript
  (|CallParentFunction))