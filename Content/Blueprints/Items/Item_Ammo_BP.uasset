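; Ammo pickup item, derived from Item_BP, that refills the player's ammo when touched.
; On sphere overlap it checks for a PlayerCharacter with room for more ammo, adds RefillAmount through the character's C++ ChangeAmmo function, then destroys itself.
; If the player's ammo is full, the pickup does nothing and stays in the world.
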(event OnComponentBeginOverlap(Sphere)
  (params (OverlappedComponent :type Primitive%20Component%20Object%20Reference) (OtherActor :type Actor%20Object%20Reference) (OtherComp :type Primitive%20Component%20Object%20Reference) (OtherBodyIndex :type Integer) (bFromSweep :type Boolean) (SweepResult :type Hit%20Result%20Structure%20%28by%20ref%29))
  ;[1 1 1] Om spilleren overlapper colission-kula...
  (if (Utilities|ClassIsChildOf (Utilities|GetClass OtherActor) "/Script/TinyDoctorTest.PlayerCharacter")
    (bind _asplayer_character (Utilities|Casting|CastToPlayerCharacter OtherActor))
    ;[1 1 1] Sjekker om spilleren har plass til mer ammo, dersom den spilleren ikke kan få mer ammo, så gjør den ingenting og kan reagere på fysikk
    (if (< (Class|PlayerCharacter|GetAmmo _asplayer_character) (Class|PlayerCharacter|GetMaxAmmo _asplayer_character))
      (Class|PlayerCharacter|ChangeAmmo _asplayer_character (Variables|Default|GetRefillAmount)) ; Gir spilleren ammo (C++)
      (Actor|DestroyActor) ; Fjerner ammo-pickupen
    )))

(fn ConstructionScript
  (|CallParentFunction) ; Arver av Item_BP
)