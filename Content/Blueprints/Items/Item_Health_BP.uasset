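; Health pickup item that restores health to a player character on contact.
; Tick bobs the static mesh vertically with a sine wave over game time and spins it around yaw at a configurable rate.
; When a PlayerCharacter overlaps the sphere and is below max health, it adds the refill amount and destroys itself, so players at full health leave it in place.
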(event OnComponentBeginOverlap(Sphere)
  (params (OverlappedComponent :type Primitive%20Component%20Object%20Reference) (OtherActor :type Actor%20Object%20Reference) (OtherComp :type Primitive%20Component%20Object%20Reference) (OtherBodyIndex :type Integer) (bFromSweep :type Boolean) (SweepResult :type Hit%20Result%20Structure%20%28by%20ref%29))
  (if (Utilities|ClassIsChildOf (Utilities|GetClass OtherActor) "/Script/TinyDoctorTest.PlayerCharacter")
    (bind _asplayer_character (Utilities|Casting|CastToPlayerCharacter OtherActor))
    (if (< (Class|Unit|GetHealth _asplayer_character) (Class|Unit|GetMaxHealth _asplayer_character))
      (Class|Unit|ChangeHealth _asplayer_character (Variables|Default|GetHealthRefill))
      (Actor|DestroyActor))))

(event EventTick
  (params (DeltaSeconds :type Float%20%28single-precision%29))
  (Transformation|SetRelativeLocation (Variables|Default|GetStaticMesh) (Math|Vector|MakeVector 0.0 0.0 (* (/ (+ (Math|Trig|Sin(Degrees) (* (Utilities|Time|GetTimeSeconds) (Variables|Default|GetFloat%20Speed))) 1.0) 2.0) (Variables|Default|GetFloat%20Height))) false false)
  (Transformation|SetRelativeRotation (Variables|Default|GetStaticMesh) (Math|Rotator|MakeRotator 0.0 0.0 (+ (.yaw (Variables|/Script/Engine.SceneComponent|GetRelativeRotation (Variables|Default|GetStaticMesh))) (* (Variables|Default|GetRotation%20Rate) (Utilities|Time|GetWorldDeltaSeconds)))) false false))

(fn ConstructionScript
  (|CallParentFunction))