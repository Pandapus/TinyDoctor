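; Player Blueprint that adds a HUD to the screen and drives a laser sight.
; On BeginPlay it creates the UITest widget, stores it as the HUD reference and adds it to the viewport.
; Each Tick, a visibility line trace from LaserSource finds the hit point, or falls back to maximum range.
; That point sets the LaserBeam target and positions LaserImpact, offset along its own forward vector.
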(event EventBeginPlay
  (bind _returnvalue (UserInterface|CreateWidget "/Game/Blueprint/UITest.UITest_C"))
  (bind _output_get (Variables|Default|SetHUD%20Reference _returnvalue))
  (UserInterface|Viewport|AddtoViewport _output_get 0))

(event Collision|EventActorBeginOverlap
  (params (OtherActor :type Actor%20Object%20Reference)))

(event EventTick
  (params (DeltaSeconds :type Float%20%28single-precision%29))
  (bind _laserimpact (Variables|Default|GetLaserImpact))
  (bind _lasersource (Variables|Default|GetLaserSource))
  (bind _laserbeam (Variables|Default|GetLaserBeam))
  (bind _returnvalue (Transformation|GetWorldLocation _lasersource))
  (bind _returnvalue_2 (Math|Vector|GetForwardVector _lasersource))
  (bind _returnvalue_3 (* _returnvalue_2 5e+03))
  (bind _returnvalue_4 (+ _returnvalue _returnvalue_3))
  ;[1 1 1] Laser sight
  (bind (_outhit _returnvalue_5) (Collision|LineTraceByChannel _returnvalue _returnvalue_4 "TraceTypeQuery1" false 0 "None"))
  (if _returnvalue_5
    (Variables|Default|SetLaserTargetLoc (.Location (Collision|BreakHitResult _outhit)))
    (else
      (Variables|Default|SetLaserTargetLoc _returnvalue_4)))
  (Class|ParticleSystemComponent|SetBeamSourcePoint _laserbeam 0 _returnvalue)
  (Class|ParticleSystemComponent|SetBeamTargetPoint _laserbeam 0 (Variables|Default|GetLaserTargetLoc))
  (Transformation|SetWorldLocation _laserimpact (- (Variables|Default|GetLaserTargetLoc) (Math|Vector|GetForwardVector _laserimpact)) false false))

(fn ConstructionScript)