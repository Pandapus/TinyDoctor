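; Ammo pickup Blueprint that refills the player's ammunition on contact.
; When a PlayerCharacter overlaps its sphere and is below max ammo, it destroys itself and grants a fixed amount of ammo.
; IncreaseAmmo adds that amount to the stored player reference's Ammo, capped at MaxAmmo.
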(event OnComponentBeginOverlap(Sphere)
  (params (OverlappedComponent :type Primitive%20Component%20Object%20Reference) (OtherActor :type Actor%20Object%20Reference) (OtherComp :type Primitive%20Component%20Object%20Reference) (OtherBodyIndex :type Integer) (bFromSweep :type Boolean) (SweepResult :type Hit%20Result%20Structure%20%28by%20ref%29))
  (bind _player_reference (Variables|Default|GetPlayer%20Reference))
  (if (Utilities|ClassIsChildOf (Utilities|GetClass OtherActor) "/Script/TinyDoctorTest.PlayerCharacter")
    (if (not (>= (Variables|/Script/TinyDoctorTest.PlayerCharacter|Getammo _player_reference) (Variables|/Script/TinyDoctorTest.PlayerCharacter|GetmaxAmmo _player_reference)))
      (CallFunction|DestroySelf)
      (CallFunction|IncreaseAmmo 5))))

(event EventTick
  (params (DeltaSeconds :type Float%20%28single-precision%29)))

(event EventBeginPlay
  (|CallParentFunction))

(fn ConstructionScript
  (|CallParentFunction))

(fn IncreaseAmmo
  (params (Amount :type Integer))
  (bind _player_reference (Variables|Default|GetPlayer%20Reference))
  (bind _player_reference_2 (Variables|Default|GetPlayer%20Reference))
  (if (> (+ Amount (Variables|/Script/TinyDoctorTest.PlayerCharacter|Getammo _player_reference)) (Variables|/Script/TinyDoctorTest.PlayerCharacter|GetmaxAmmo _player_reference))
    (Variables|/Script/TinyDoctorTest.PlayerCharacter|Setammo _player_reference_2 (Variables|/Script/TinyDoctorTest.PlayerCharacter|GetmaxAmmo _player_reference_2))
    (else
      (Variables|/Script/TinyDoctorTest.PlayerCharacter|Setammo (Variables|Default|GetPlayer%20Reference) (+ Amount (Variables|/Script/TinyDoctorTest.PlayerCharacter|Getammo (Variables|Default|GetPlayer%20Reference)))))))