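; Health pickup item that heals the player when they walk into it.
; On sphere overlap by a PlayerCharacter, it checks whether the stored player reference is below max health.
; If so, it destroys itself and then adds HealthRefill to the player's health; at full health it stays in the world.
; BeginPlay and construction defer to the parent pickup class.
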(event OnComponentBeginOverlap(Sphere)
  (params (OverlappedComponent :type Primitive%20Component%20Object%20Reference) (OtherActor :type Actor%20Object%20Reference) (OtherComp :type Primitive%20Component%20Object%20Reference) (OtherBodyIndex :type Integer) (bFromSweep :type Boolean) (SweepResult :type Hit%20Result%20Structure%20%28by%20ref%29))
  (bind _player_reference (Variables|Default|GetPlayer%20Reference))
  (if (Utilities|ClassIsChildOf (Utilities|GetClass OtherActor) "/Script/TinyDoctorTest.PlayerCharacter")
    (if (< (Class|Unit|GetHealth _player_reference) (Class|Unit|GetMaxHealth _player_reference))
      (CallFunction|DestroySelf)
      (Class|Unit|ChangeHealth (Variables|Default|GetPlayer%20Reference) (Variables|Default|GetHealthRefill)))))

(event EventBeginPlay
  (|CallParentFunction))

(fn ConstructionScript
  (|CallParentFunction))