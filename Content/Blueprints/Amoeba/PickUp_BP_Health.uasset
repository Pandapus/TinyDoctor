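; Health pickup that restores one point of the player's health on contact and then removes itself.
; A sphere overlap checks that the other actor is a PlayerCharacter and that PlayerReference is below maximum health, so the pickup remains when health is full.
; It calls DestroySelf, then IncreaseHealth, which adds the amount to PlayerReference's health and caps it at MaxHealth.
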(event OnComponentBeginOverlap(Sphere)
  (params (OverlappedComponent :type Primitive%20Component%20Object%20Reference) (OtherActor :type Actor%20Object%20Reference) (OtherComp :type Primitive%20Component%20Object%20Reference) (OtherBodyIndex :type Integer) (bFromSweep :type Boolean) (SweepResult :type Hit%20Result%20Structure%20%28by%20ref%29))
  (bind _player_reference (Variables|Default|GetPlayer%20Reference))
  (if (Utilities|ClassIsChildOf (Utilities|GetClass OtherActor) "/Script/TinyDoctorTest.PlayerCharacter")
    (if (not (>= (Variables|/Script/TinyDoctorTest.Unit|Gethealth _player_reference) (Variables|/Script/TinyDoctorTest.Unit|GetmaxHealth _player_reference)))
      (CallFunction|DestroySelf)
      (CallFunction|IncreaseHealth 1.0))))

(event EventBeginPlay
  (|CallParentFunction))

(fn ConstructionScript
  (|CallParentFunction))

(fn IncreaseHealth
  (params (Amount :type Float%20%28single-precision%29))
  (bind _player_reference (Variables|Default|GetPlayer%20Reference))
  (bind _player_reference_2 (Variables|Default|GetPlayer%20Reference))
  (if (> (+ (Variables|/Script/TinyDoctorTest.Unit|Gethealth _player_reference_2) Amount) (Variables|/Script/TinyDoctorTest.Unit|GetmaxHealth _player_reference_2))
    (Variables|/Script/TinyDoctorTest.Unit|Sethealth _player_reference (Variables|/Script/TinyDoctorTest.Unit|GetmaxHealth _player_reference))
    (else
      (Variables|/Script/TinyDoctorTest.Unit|Sethealth (Variables|Default|GetPlayer%20Reference) (+ Amount (Variables|/Script/TinyDoctorTest.Unit|Gethealth (Variables|Default|GetPlayer%20Reference)))))))