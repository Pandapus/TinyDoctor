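; Pickup actor that bobs up and down and destroys itself when a PlayerCharacter overlaps it.
; Each tick adds a sine offset based on real time to the current Z position, so the bob's amplitude depends on frame rate.
; The overlap handler only checks the other actor's class and destroys the pickup, granting nothing to the player.
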(event EventBeginPlay)

(event Collision|EventActorBeginOverlap
  (params (OtherActor :type Actor%20Object%20Reference))
  (if (Utilities|ClassIsChildOf (Utilities|GetClass OtherActor) "/Script/TinyDoctorTest.PlayerCharacter")
    (Actor|DestroyActor)))

(event EventTick
  (params (DeltaSeconds :type Float%20%28single-precision%29))
  (Transformation|SetActorLocation (+ (Transformation|GetActorLocation) (Math|Vector|MakeVector 0.0 0.0 (* (Math|Trig|Sin(Degrees) (* (Utilities|Time|GetRealTimeSeconds) 2e+02)) 5.0))) false false))

(fn ConstructionScript)