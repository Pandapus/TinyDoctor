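; AI controller for the Amoeba pawn that starts its behavior tree on BeginPlay.
; It loads the Amoeba blackboard and stores the pawn's spawn location as OriginalPosition.
; It copies the Amoeba's DetectionRadius into the blackboard, then runs AmoebaBehaviourTree; a pawn of another class stops setup before the tree runs.
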(event EventBeginPlay
  (bind _blackboardcomponent (Class|AIController|UseBlackboard "/Game/Blueprints/Amoeba/AmoebaBlackboard.AmoebaBlackboard"))
  ;[1 1 1] Set Original Position
  (AI|Components|Blackboard|SetValueasVector _blackboardcomponent (Utilities|Name|MakeLiteralName "OriginalPosition") (Transformation|GetActorLocation (Pawn|GetControlledPawn)))
  ;[1 1 1] Set Detection Radius
  (bind _asamoeba (Utilities|Casting|CastToAmoeba (Pawn|GetControlledPawn)))
  (AI|Components|Blackboard|SetValueasFloat _blackboardcomponent (Utilities|Name|MakeLiteralName "DetectionRadius") (Variables|/Script/TinyDoctorTest.Amoeba|GetdetectionRadius _asamoeba))
  (AI|RunBehaviorTree "/Game/Blueprints/Amoeba/AmoebaBehaviourTree.AmoebaBehaviourTree"))

(fn ConstructionScript)