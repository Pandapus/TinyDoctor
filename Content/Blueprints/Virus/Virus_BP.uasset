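; Virus enemy character that chases the player, leaps at them and destroys itself on contact to deal damage.
; When the player enters its detection radius, it tells its spawner to start the chase.
; While chasing, it launches itself toward the player when close and grounded.
; On destruction it leaves the spawner's array, destroying the spawner once none remain.
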(event OnComponentHit(CapsuleComponent)
  (params (HitComponent :type Primitive%20Component%20Object%20Reference) (OtherActor :type Actor%20Object%20Reference) (OtherComp :type Primitive%20Component%20Object%20Reference) (NormalImpulse :type Vector :default "0, 0, 0") (Hit :type Hit%20Result%20Structure%20%28by%20ref%29))
  (if (Utilities|ClassIsChildOf (Utilities|GetClass OtherActor) "/Script/TinyDoctorTest.PlayerCharacter")
    (bind _asunit (Utilities|Casting|CastToUnit OtherActor))
    (Class|Unit|DecreaseHealth _asunit (Variables|Default|GetDamage))
    (Actor|DestroyActor)))

(event EventTick
  (params (DeltaSeconds :type Float%20%28single-precision%29))
  (bind _returnvalue (Game|Player|GetPlayerPawn 0))
  (bind _returnvalue_2 (Transformation|GetActorLocation))
  (bind _horizontal_jump_strength (Variables|Default|GetHorizontal%20Jump%20Strength))
  (bind _returnvalue_3 (Transformation|GetActorLocation _returnvalue))
  (bind _returnvalue_4 (- _returnvalue_3 _returnvalue_2))
  (bind _returnvalue_5 (Math|Vector|Normalize _returnvalue_4))
  (bind (_x _y) (Math|Vector|BreakVector _returnvalue_5))
  (if (Variables|Default|GetbChasingPlayer)
    ;[1 1 1] Jump Towards Player
    (if (<= (Math|Vector|VectorLength (- (Transformation|GetActorLocation (Game|Player|GetPlayerPawn 0)) (Transformation|GetActorLocation))) (Math|Float|MakeLiteralFloat 5e+02))
      (if (AI|Components|NavMovement|IsMovingonGround (Variables|Character|GetCharacterMovement))
        (Character|LaunchCharacter (Math|Vector|MakeVector (* _x _horizontal_jump_strength) (* _y _horizontal_jump_strength) (Variables|Default|GetVertical%20Jump%20Strength)) true true)))
    (elif (<= (Math|Vector|VectorLength (- (Transformation|GetActorLocation (Game|Player|GetPlayerPawn 0)) (Transformation|GetActorLocation))) (Variables|Default|GetdetectionRadius))
      (Class|VirusSpawner|ChasePlayer (Variables|Default|GetSpawnerRef)))))

(event EventDestroyed
  (bind _spawnerref (Variables|Default|GetSpawnerRef))
  (bind _virusarray (Variables|/Script/TinyDoctorTest.VirusSpawner|GetvirusArray _spawnerref))
  (Utilities|Array|RemoveItem _virusarray self)
  (if (<= (Utilities|Array|Length _virusarray) 0)
    (Actor|DestroyActor (Variables|Default|GetSpawnerRef))))

(fn ConstructionScript)