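; Amoeba enemy Blueprint that drops ammo pickups when destroyed.
; Its Destroyed event spawns zero to two PickUp_BP_Ammo actors at random horizontal offsets around its location, regardless of collision.
; Each pickup's mesh receives an upward force with random sideways scatter, applied as a mass-independent acceleration change.
; The Blueprint contains no other logic, and its construction script is empty.
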(event EventDestroyed
  (bind _returnvalue (Transformation|GetActorLocation))
  (bind (_x _y _z) (Math|Vector|BreakVector _returnvalue))
  (for _index (range 1 (Math|Random|RandomIntegerinRange 0 2))
    (bind _returnvalue_2 (Game|SpawnActorfromClass "/Game/Blueprints/Items/PickUp_BP_Ammo.PickUp_BP_Ammo_C" (Math|Conversions|ToTransform(Vector) (Math|Vector|MakeVector (+ _x (Math|Random|RandomFloatinRange -1e+02 1e+02)) (+ _y (Math|Random|RandomFloatinRange -1e+02 1e+02)) _z)) "AlwaysSpawn" 0 0 0))
    (Physics|AddForce (Variables|/Game/Blueprints/Items/PickUp_BP.PickUp_BP_C|GetStatic%20Mesh _returnvalue_2) (* (Math|Vector|MakeVector (Math|Random|RandomFloatinRange -5e+02 5e+02) (Math|Random|RandomFloatinRange -5e+02 5e+02) 5e+02) 1e+02) "None" true)))

(fn ConstructionScript)