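; Boss minion spawner that spawns chasing enemies at its own transform for a boss fight.
; StartSpawning sets the amount and resets the counter, then Tick spawns until that amount is reached, pausing between spawns with a flag and Delay.
; Each spawn randomly picks an Amoeba or a VirusSpawner, starts its chase behavior and adds it to the SpawnedEnemies list on the BossAIController cached at BeginPlay.
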(event EventTick
  (params (DeltaSeconds :type Float%20%28single-precision%29))
  (bind _returnvalue (Transformation|GetActorTransform))
  (if (not (Variables|Default|GetCurrently%20Spawning))
    (if (< (Variables|Default|GetEnemies%20Spawned) (Variables|Default|GetAmount%20To%20Spawn))
      (switch int (Math|Random|RandomInteger 2)
        (:0
          (bind _returnvalue_2 (Game|SpawnActorfromClass "/Game/Blueprints/Amoeba/Amoeba_BP.Amoeba_BP_C" _returnvalue "AdjustIfPossibleButAlwaysSpawn" 0 0))
          (bind _asamoeba_aicontroller (Utilities|Casting|CastToAmoebaAIController (Pawn|GetController _returnvalue_2)))
          (Class|AmoebaAIController|StartChaseMode _asamoeba_aicontroller)
          (Utilities|Array|Add (Variables|/Script/TinyDoctorTest.BossAIController|GetspawnedEnemies (Variables|Default|GetBossRef)) _returnvalue_2))
        (:1
          (bind _returnvalue_3 (Game|SpawnActorfromClass "/Game/Blueprints/Virus/VirusSpawner_BP.VirusSpawner_BP_C" _returnvalue "AdjustIfPossibleButAlwaysSpawn" 0 0))
          (Class|VirusSpawner|ChasePlayer _returnvalue_3)
          (Utilities|Array|Add (Variables|/Script/TinyDoctorTest.BossAIController|GetspawnedEnemies (Variables|Default|GetBossRef)) _returnvalue_3)))
      (Variables|Default|SetCurrently%20Spawning true)
      (Utilities|FlowControl|Delay (Variables|Default|GetTime%20Between%20Spawns))
      (Variables|Default|SetCurrently%20Spawning false)
      (Math|Integer|IncrementInt (Variables|Default|GetEnemies%20Spawned)))))

(event EventBeginPlay
  (bind _asboss_aicontroller (Utilities|Casting|CastToBossAIController (Variables|Default|GetbossActorReference)))
  (bind _output_get (Variables|Default|SetBossRef _asboss_aicontroller))
  (Utilities|IsValid _output_get
    (:Is%20Not%20Valid
      (Development|PrintString "Boss Ref Not Valid"))))

(event EventStartSpawning
  (params (amountToSpawn :type Integer))
  (CallFunction|StartSpawning amountToSpawn))

(fn ConstructionScript)

(fn StartSpawning
  (params (Amount%20To%20Spawn :type Integer))
  (Variables|Default|SetAmount%20To%20Spawn Amount%20To%20Spawn)
  (Variables|Default|SetEnemies%20Spawned 0)
  (Variables|Default|SetCurrently%20Spawning false))