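; Player Blueprint that drives a laser sight and a shotgun attack.
; Each tick, a trace from LaserSource sets the laser beam's endpoints and places the impact marker.
; Shotgun spends ammo, then fires a horizontal fan of debug-drawn traces around the actor's forward vector by cumulatively rotating it about Z.
; Each trace hitting a Unit applies damage with knockback from the hit location.
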(event EventTick
  (params (DeltaSeconds :type Float%20%28single-precision%29))
  (bind _laserimpact (Variables|Default|GetLaserImpact))
  (bind _lasersource (Variables|Default|GetLaserSource))
  (bind _laserbeam (Variables|Default|GetLaserBeam))
  (bind _returnvalue (Transformation|GetWorldLocation _lasersource))
  (bind _returnvalue_2 (Math|Vector|GetForwardVector _lasersource))
  (bind _returnvalue_3 (* _returnvalue_2 5e+03))
  (bind _returnvalue_4 (+ _returnvalue _returnvalue_3))
  ;[1 1 1] Laser sight
  (bind (_outhit _returnvalue_5) (Collision|LineTraceByChannel _returnvalue _returnvalue_4 "TraceTypeQuery1" false 0 "None"))
  (if _returnvalue_5
    (Variables|Shotgun|SetLaserTargetLoc (.Location (Collision|BreakHitResult _outhit)))
    (else
      (Variables|Shotgun|SetLaserTargetLoc _returnvalue_4)))
  (Class|ParticleSystemComponent|SetBeamSourcePoint _laserbeam 0 _returnvalue)
  (Class|ParticleSystemComponent|SetBeamTargetPoint _laserbeam 0 (Variables|Shotgun|GetLaserTargetLoc))
  (Transformation|SetWorldLocation _laserimpact (- (Variables|Shotgun|GetLaserTargetLoc) (Math|Vector|GetForwardVector _laserimpact)) false false))

(event EventShotgun
  (bind _lasersource (Variables|Default|GetLaserSource))
  (bind _returnvalue (Transformation|GetWorldLocation _lasersource))
  ;[1 1 1] Shotgun
  (if (>= (Class|PlayerCharacter|GetAmmo) (Variables|Shotgun|GetShotgun%20Ammo%20Cost))
    (Class|PlayerCharacter|DecreaseAmmo (Variables|Shotgun|GetShotgun%20Ammo%20Cost))
    (Variables|Shotgun|SetShotgunLineTraceVector (* (Transformation|GetActorForwardVector) (Variables|Shotgun|GetShotgunDistance)))
    (for _index (range 1 (Variables|Shotgun|GetShotgunLinetraces))
      (if (== _index 1)
        (Variables|Shotgun|SetShotgunLineTraceVector (Math|Vector|RotateVectorAroundAxis (Variables|Shotgun|GetShotgunLineTraceVector) (* (* (Variables|Shotgun|GetShotgun%20Spread) (/ (Math|Conversions|ToFloat(Integer) (Variables|Shotgun|GetShotgunLinetraces)) 2.0)) -1.0) (Math|Vector|MakeVector 0.0 0.0 1.0)))
        (else
          (Variables|Shotgun|SetShotgunLineTraceVector (Math|Vector|RotateVectorAroundAxis (Variables|Shotgun|GetShotgunLineTraceVector) (Variables|Shotgun|GetShotgun%20Spread) (Math|Vector|MakeVector 0.0 0.0 1.0)))))
      (bind _outhit (Collision|LineTraceByChannel _returnvalue (+ _returnvalue (Variables|Shotgun|GetShotgunLineTraceVector)) "TraceTypeQuery1" false 0 "ForDuration" true "(R=1.000000,G=0.000000,B=0.000000,A=1.000000)" "(R=0.000000,G=1.000000,B=0.000000,A=1.000000)" 1.0))
      (if (Utilities|ClassIsChildOf (Utilities|GetClass (.HitActor (Collision|BreakHitResult _outhit))) "/Script/TinyDoctorTest.Unit")
        (bind _asunit (Utilities|Casting|CastToUnit (.HitActor (Collision|BreakHitResult _outhit))))
        (Class|Unit|TakeDamagewithKnockback _asunit 1.0 (.Location (Collision|BreakHitResult _outhit)) 1e+03 1e+03)))))

(fn ConstructionScript)